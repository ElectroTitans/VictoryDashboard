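; VictoryConnectUtil is a utility Blueprint that parses a raw text message into VictoryConnect packet fields.
; Parse uses chained string splits to extract an integer subject, a two-value packet type selected by integer, and a topic string.
; It takes the brace-enclosed remainder and breaks it on semicolons into the packet data array, dropping empty entries.
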(fn `Parse`
  (params (InText :type String))
  (returns (Packet :type "/Game/Blueprints/VictoryConnectPacket Structure"))
  (bind (_lefts _rights) (`KismetStringLibrary.Split` InText " "))
  (bind (_lefts_2 _rights_2) (`KismetStringLibrary.Split` _rights " "))
  (bind (_lefts_3 _rights_3) (`KismetStringLibrary.Split` _rights_2 " "))
  (return (make `/Game/Blueprints/VictoryConnectPacket` (`KismetStringLibrary.Conv_StringToInt` _lefts) (select `int` (`KismetStringLibrary.Conv_StringToInt` _lefts_2) :`0` "NewEnumerator0" :`1` "NewEnumerator1" :!type "/Game/Blueprints/VictoryConnectMessageType Enum") _lefts_3 (`KismetStringLibrary.ParseIntoArray` (`KismetStringLibrary.GetSubstring` _rights_3 (+ (`KismetStringLibrary.FindSubstring` _rights_3 "{") 1) (- (`KismetStringLibrary.FindSubstring` _rights_3 "}") 1)) ";"))))