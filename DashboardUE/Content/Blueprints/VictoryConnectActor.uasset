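; VictoryConnectActor is a TCP client that links the game to a local message server, identifying itself as VictoryDash.
; It connects on BeginPlay, retries after a short delay on failure, and reports each connection stage through a dispatcher.
; Incoming text is parsed and broadcast through a topic dispatcher, and heartbeat requests are answered automatically.
; Subscribe sends topic subscription messages, while BindTopic is an empty stub.
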(event `self.ReceiveBeginPlay`
  (`self.Connect` "127.0.0.1"))

(event `Connect`
  (params (IP :type String))
  (bind _returnvalue (`SocketClientHandler.getSocketClientTarget`))
  (`self.ConnectionDispatcher` "NewEnumerator0")
  (bind _output_get (set `self.IP` IP))
  (`SocketClientBPLibrary.connectSocketClient` _returnvalue _output_get 5800)
  (add `SocketClientBPLibrary.onsocketClientConnectionEventDelegate` _returnvalue (delegate `ConnectStatus`)))

(event `ConnectStatus`
  (params (success :type Boolean) (message :type String))
  (`KismetSystemLibrary.PrintString` message)
  (if success
    (add `SocketClientBPLibrary.onreceiveTCPMessageEventDelegate` (`SocketClientHandler.getSocketClientTarget`) (delegate `OnTCPData`))
    (`SocketClientBPLibrary.socketClientSendTCPMessage` "0 0 id {VictoryDash}")
    (`self.ConnectionDispatcher` "NewEnumerator2")
    (else
      (`self.ConnectionDispatcher` "NewEnumerator1")
      (`KismetSystemLibrary.Delay` 0.1)
      (`self.Connect` (`self.IP`)))))

(event `OnTCPData`
  (params (message :type String))
  (bind _packet (`/Game/Blueprints/VictoryConnectUtil.Parse` message))
  (`self.TopicDispatcher` _packet)
  (bind (_subject _type _topic) (break `/Game/Blueprints/VictoryConnectPacket` _packet))
  (switch `/Game/Blueprints/VictoryConnectMessageType` _type
    (:`NewEnumerator1`
      (switch `string` _topic
        (:`heartbeat`
          (`SocketClientBPLibrary.socketClientSendTCPMessage` "0 0 heartbeat {no_data}"))))))

(event `BindTopic`
  (params (NewParam :type Boolean)))

(event `Subscribe`
  (params (Topic :type String))
  (`SocketClientBPLibrary.socketClientSendTCPMessage` (`KismetStringLibrary.Concat_StrStr` "0 0 subscribe {" Topic "}")))

(fn `UserConstructionScript`)