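; Robot actor that mirrors live telemetry from an external robot through the VictoryConnect actor.
; On BeginPlay it binds to that actor's topic and connection dispatchers, then subscribes to the motors and navx topics once connected.
; Navx packets set the Cube's world yaw.
; Motors packets write four drive values (LF, LR, RF, RR) to text displays.
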(event `self.ReceiveBeginPlay`
  (bind _newparam3 (`/Game/Blueprints/VictoryConnectMacro_Actor.GetVictoryConnectActor`)
    (:`NewParam2`
      (add `/Game/Blueprints/VictoryConnectActor.TopicDispatcher` _newparam3 (delegate `Topic`))
      (add `/Game/Blueprints/VictoryConnectActor.ConnectionDispatcher` _newparam3 (delegate `Con`)))))

(event `Con`
  (params (Success :type "/Game/Blueprints/ConnectionStatus Enum" :default "NewEnumerator0"))
  (switch `/Game/Blueprints/ConnectionStatus` Success
    (:`NewEnumerator2`
      (`/Game/Blueprints/VictoryConnectActor.Subscribe` (stale `self.ReceiveBeginPlay` _newparam3) "motors")
      (`/Game/Blueprints/VictoryConnectActor.Subscribe` (stale `self.ReceiveBeginPlay` _newparam3) "navx"))))

(event `Topic`
  (params (Packet :type "/Game/Blueprints/VictoryConnectPacket Structure"))
  (switch `string` Packet_Topic_13_7B7E3735426A7C9BC003AABAE5F78F28
    (:`navx`
      (`SceneComponent.K2_SetWorldRotation` (`self.Cube`) (`KismetMathLibrary.MakeRotator` 0.0 0.0 (`KismetStringLibrary.Conv_StringToDouble` (`|GetArrayItem` Packet_Data_25_F9D6C72D481AABBBB2931DBF06D1834D 1))) false false))
    (:`motors`
      (`TextRenderComponent.K2_SetText` (`self.DriveLF`) (`KismetTextLibrary.Conv_StringToText` (`|GetArrayItem` Packet_Data_25_F9D6C72D481AABBBB2931DBF06D1834D)))
      (`TextRenderComponent.K2_SetText` (`self.DriveLR`) (`KismetTextLibrary.Conv_StringToText` (`|GetArrayItem` Packet_Data_25_F9D6C72D481AABBBB2931DBF06D1834D 1)))
      (`TextRenderComponent.K2_SetText` (`self.DriveRF`) (`KismetTextLibrary.Conv_StringToText` (`|GetArrayItem` Packet_Data_25_F9D6C72D481AABBBB2931DBF06D1834D 2)))
      (`TextRenderComponent.K2_SetText` (`self.DriveRR`) (`KismetTextLibrary.Conv_StringToText` (`|GetArrayItem` Packet_Data_25_F9D6C72D481AABBBB2931DBF06D1834D 3))))))

(event `self.ReceiveTick`
  (params (DeltaSeconds :type "Float (single-precision)")))

(fn `UserConstructionScript`)