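; Socket client actor that links a Victory dashboard to a TCP server and reports connection state and raw traffic to the UI_Main widget it spawns.
; StartVictoryConnect connects on a fixed port using a manual IP (the non-manual branch is empty), retrying after a delay on failure.
; Incoming messages are parsed by type and topic, answering Welcome with a dashboard ID and Heartbeat requests with a keep-alive.
; EndPlay closes the socket.
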(event `self.ReceiveBeginPlay`
  (bind _returnvalue (`|CreateWidget` "/Game/UI/UI_Main.UI_Main_C" (`GameplayStatics.GetPlayerController` 0)))
  (`UserWidget.AddToViewport` _returnvalue 0)
  (set `self.UI` _returnvalue))

(event `AttemptReconnect`
  (bind _returnvalue (`SocketClientHandler.getSocketClientTarget`))
  (`SocketClientBPLibrary.connectSocketClient` _returnvalue (stale `StartVictoryConnect` _output_get) 9000 :!label _label)
  (add `SocketClientBPLibrary.onsocketClientConnectionEventDelegate` _returnvalue (delegate `TCPStatus`))
  (message `/Game/Blueprints/VictoryConnectInterface.OnConnecting` (`self.UI`)))

(event `StartVictoryConnect`
  (params (`IP/TeamNumber` :type String) (`Manual IP` :type Boolean))
  (if `Manual IP`
    (bind _output_get (set `self.FormatedIP` `IP/TeamNumber`))
    (goto _label)))

(event `TCPStatus`
  (params (success :type Boolean) (message :type String))
  (bind _ui (`self.UI`))
  (message `/Game/Blueprints/VictoryConnectInterface.OnRawData` (`self.UI`) message)
  (if success
    (add `SocketClientBPLibrary.onreceiveTCPMessageEventDelegate` (`SocketClientHandler.getSocketClientTarget`) (delegate `TCPData`))
    (`/Game/UI/UI_Main.OnConnected` _ui)
    (else
      (message `/Game/Blueprints/VictoryConnectInterface.OnFailedConnect` _ui)
      (`KismetSystemLibrary.Delay` 3.0)
      (`self.AttemptReconnect`))))

(event `TCPData`
  (params (message :type String))
  (bind _returnvalue (`KismetStringLibrary.BuildString_Int` "" "" (`self.ID`) " 0 id victory_dashboard"))
  (message `/Game/Blueprints/VictoryConnectInterface.OnRawData` (`self.UI`) message)
  (bind _packet (`/Game/Blueprints/VictoryConnectLib.Parse` message))
  (set `self.ID` (break `/Game/Blueprints/VictoryConnectPacket` _packet))
  (switch `/Game/Blueprints/VictoryConnectMessageType` (`.Type_6_5A42DB5E4F2B48CA32E21E9CFCD82ED2` (break `/Game/Blueprints/VictoryConnectPacket` _packet))
    (:`NewEnumerator0`
      (switch `string` (`.Topic_13_7B7E3735426A7C9BC003AABAE5F78F28` (break `/Game/Blueprints/VictoryConnectPacket` _packet))
        (:`welcome`
          (`KismetSystemLibrary.Delay` 0.2)
          (`SocketClientBPLibrary.socketClientSendTCPMessage` (`SocketClientHandler.getSocketClientTarget`) _returnvalue true)
          (message `/Game/Blueprints/VictoryConnectInterface.OnRawData` (`self.UI`) (`KismetStringLibrary.Concat_StrStr` "Sending -> " _returnvalue)))))
    (:`NewEnumerator1`
      (switch `string` (`.Topic_13_7B7E3735426A7C9BC003AABAE5F78F28` (break `/Game/Blueprints/VictoryConnectPacket` _packet))
        (:`heartbeat`
          (`SocketClientBPLibrary.socketClientSendTCPMessage` (`SocketClientHandler.getSocketClientTarget`) (`KismetStringLibrary.BuildString_Int` "" "" (`self.ID`) " 0 heartbeat no_data") true))))))

(event `self.ReceiveEndPlay`
  (params (EndPlayReason :type "EEndPlayReason Enum" :default "Destroyed"))
  (`SocketClientBPLibrary.closeSocketClientConnection` (`SocketClientHandler.getSocketClientTarget`)))

(fn `UserConstructionScript`)